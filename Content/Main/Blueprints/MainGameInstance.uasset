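; Game instance Blueprint that shows the main menu and starts a new game.
; ShowMainMenu creates and caches the MainMenu widget behind a validity check, adds it to the viewport, shows the cursor and sets UI-only input locked in fullscreen.
; CreateNewGame keeps the cursor visible, switches to game-and-UI input and opens the MountainVillage level by name.
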(event Custom|Show%20Main%20Menu
  (bind _returnvalue (Game|GetPlayerController 0))
  (Utilities|IsValid 0
    (:Is%20Valid
      _)
    (:Is%20Not%20Valid
      (bind _returnvalue_2 (UserInterface|CreateWidget "/Game/Main/Blueprints/MainMenu/Widget/MainMenu.MainMenu_C" _returnvalue))
      (Variables|Default|SetMainMenuWB _returnvalue_2)))
  (UserInterface|Viewport|AddtoViewport (Variables|Default|GetMainMenuWB) 0)
  (Variables|/Script/Engine.PlayerController|SetbShowMouseCursor _returnvalue true)
  (Input|SetInputModeUIOnly _returnvalue (Variables|Default|GetMainMenuWB) "LockInFullscreen" false))

(event Custom|Create%20New%20Game
  (bind _returnvalue (Game|GetPlayerController 0))
  (Variables|/Script/Engine.PlayerController|SetbShowMouseCursor _returnvalue true)
  (Input|SetInputModeGameandUI _returnvalue 0 "DoNotLock" true false)
  (Game|OpenLevel(byName) "MountainVillage"))